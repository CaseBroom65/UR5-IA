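; Door actor that opens once enough items have been collected.
; Each CollectItem call increments a counter and runs a check against MaxItem, with a DoOnce so the open triggers a single time.
; Opening waits on a short delay, then snaps the Cube component to a lowered relative location without sweep or animation.
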(event `Open_Door`
  (`KismetSystemLibrary.Delay` 3.0)
  (`SceneComponent.K2_SetRelativeLocation` (`self.Cube`) (0.0 0.0 -120.0) false false))

(event `Collect Item`
  (`/Engine/EditorBlueprintResources/StandardMacros.IncrementInt` (`self.currenItemCollected`)
    (:`  `
      (`self.Open_Door_Check`))))

(event `Open_Door_Check`
  (if (>= (`self.currenItemCollected`) (`self.MaxItem`))
    (`/Engine/EditorBlueprintResources/StandardMacros.DoOnce` false
      (:`Completed`
        (`self.Open_Door`)))))

(fn `UserConstructionScript`)