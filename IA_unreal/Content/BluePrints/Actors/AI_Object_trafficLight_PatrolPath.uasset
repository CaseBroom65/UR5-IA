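; Traffic light actor that cycles between red and green lamps once something overlaps its Box component.
; The overlap calls ChangeLight, which swaps lit and glass materials on the RedLight and GreenLight components, starting with red.
; ChangeLight calls itself after timed Delays, so the cycle repeats with no stop condition or guard against repeated overlaps.
; The changes are purely visual, with no patrol or AI logic in these graphs.
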(event `self.Box.OnComponentBeginOverlap`
  (params (OverlappedComponent :type "PrimitiveComponent Object Reference") (OtherActor :type "Actor Object Reference") (OtherComp :type "PrimitiveComponent Object Reference") (OtherBodyIndex :type Integer) (bFromSweep :type Boolean) (SweepResult :type "HitResult Structure (by ref)"))
  (`self.ChangeLight`))

(event `ChangeLight`
  (`PrimitiveComponent.SetMaterial` (`self.RedLight`) 0 "/Game/Assets/textures/Red_Stop.Red_Stop")
  (`PrimitiveComponent.SetMaterial` (`self.GreenLight`) 0 "/Game/MAterials/Glass_mat_Inst.Glass_mat_Inst")
  (`KismetSystemLibrary.Delay` 2.0)
  (`PrimitiveComponent.SetMaterial` (`self.RedLight`) 0 "/Game/MAterials/Glass_mat.Glass_mat")
  (`PrimitiveComponent.SetMaterial` (`self.GreenLight`) 0 "/Game/Assets/textures/Green_light.Green_light")
  (`KismetSystemLibrary.Delay` 2.0)
  (`self.ChangeLight`))

(fn `UserConstructionScript`
  (`parent.UserConstructionScript`))