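; Rope swing actor that the player grabs, swings on and climbs after overlapping its box enables input.
; Holding Space attaches the character to the cable's end socket and moves this actor to them; releasing detaches and launches them.
; WASD sets world-axis cable force, while E and Q climb up and down through delay loops, both checked against the top marker's height.
; The construction script positions top and bottom markers.
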(event `self.Box.OnComponentBeginOverlap`
  (params (OverlappedComponent :type "PrimitiveComponent Object Reference") (OtherActor :type "Actor Object Reference") (OtherComp :type "PrimitiveComponent Object Reference") (OtherBodyIndex :type Integer) (bFromSweep :type Boolean) (SweepResult :type "HitResult Structure (by ref)"))
  ;[1 1 1] Enable Input
  (`self.EnableInput` self (`GameplayStatics.GetPlayerController` 0)))

(event `Key|SpaceBar`
  (params (Key :type "Key Structure"))
  (bind _returnvalue (`GameplayStatics.GetPlayerCharacter` 0))
  (bind (_returnvalue_x _returnvalue_y) (`KismetMathLibrary.BreakVector` (`self.K2_GetActorLocation` _returnvalue)))
  (bind _charactermovement (`Character.CharacterMovement` _returnvalue))
  ;[1 1 1] getting on and off rope
  (:`Pressed`
    (set `self.player Height` (.z (.location (`self.GetTransform` (`GameplayStatics.GetPlayerCharacter` 0)))))
    (`self.K2_AttachToActor` _returnvalue (`self.cable ref`) "CableEnd" "SnapToTarget" "KeepWorld" "KeepWorld" true)
    (`self.K2_SetActorLocation` (`KismetMathLibrary.MakeVector` _returnvalue_x _returnvalue_y (`self.player Height`)))
    (`CharacterMovementComponent.SetMovementMode` _charactermovement "MOVE_None" 0))
  (:`Released`
    (`self.K2_DetachFromActor` _returnvalue "KeepWorld" "KeepWorld" "KeepWorld")
    (`CharacterMovementComponent.SetMovementMode` _charactermovement "MOVE_Falling" 0)
    (`Character.LaunchCharacter` _returnvalue (+ (* (`self.GetActorForwardVector` _returnvalue) 300.0) (* (`self.GetActorUpVector` _returnvalue) 50.0)) false false)
    (`self.DisableInput` self (`GameplayStatics.GetPlayerController` 0))))

(event `Key|W`
  (params (Key :type "Key Structure"))
  ;[1 1 1] Swing rope
  (:`Pressed`
    (set `CableComponent.CableForce` (100.0 0.0 0.0) (`CableActor.CableComponent` (`self.cable ref`)))))

(event `Key|A`
  (params (Key :type "Key Structure"))
  ;[1 1 1] Swing rope
  (:`Pressed`
    (set `CableComponent.CableForce` (0.0 100.0 0.0) (`CableActor.CableComponent` (`self.cable ref`)))))

(event `Key|E`
  (params (Key :type "Key Structure"))
  (bind (_returnvalue_x _returnvalue_y _returnvalue_z) (`KismetMathLibrary.BreakVector` (`SceneComponent.K2_GetComponentLocation` (`self.top clif ref`))))
  (bind (_returnvalue_x_2 _returnvalue_y_2 _returnvalue_z_2) (`KismetMathLibrary.BreakVector` (`self.K2_GetActorLocation` (`GameplayStatics.GetPlayerCharacter` 0))))
  ;[1 1 1] Climb up and down
  (:`Pressed`
    (set `self.eHeld_0` true)
    (if (>= _returnvalue_z _returnvalue_z_2) :!label _label
      (`self.K2_AddActorWorldOffset` (`GameplayStatics.GetPlayerCharacter` 0) (0.0 0.0 10.0) false false)
      (`KismetSystemLibrary.Delay` 0.2)
      (if (`self.eHeld_0`)
        (goto _label))))
  (:`Released`
    (set `self.eHeld_0` false)))

(event `Key|S`
  (params (Key :type "Key Structure"))
  ;[1 1 1] Swing rope
  (:`Pressed`
    (set `CableComponent.CableForce` (-100.0 0.0 0.0) (`CableActor.CableComponent` (`self.cable ref`)))))

(event `Key|D`
  (params (Key :type "Key Structure"))
  ;[1 1 1] Swing rope
  (:`Pressed`
    (set `CableComponent.CableForce` (0.0 -100.0 0.0) (`CableActor.CableComponent` (`self.cable ref`)))))

(event `Key|Q`
  (params (Key :type "Key Structure"))
  (bind (_returnvalue_x _returnvalue_y _returnvalue_z) (`KismetMathLibrary.BreakVector` (`SceneComponent.K2_GetComponentLocation` (`self.top clif ref`))))
  (bind (_returnvalue_x_2 _returnvalue_y_2 _returnvalue_z_2) (`KismetMathLibrary.BreakVector` (`self.K2_GetActorLocation` (`GameplayStatics.GetPlayerCharacter` 0))))
  ;[1 1 1] Climb up and down
  (:`Pressed`
    (set `self.qHeld` true)
    (if (<= _returnvalue_z _returnvalue_z_2) :!label _label_2
      (`self.K2_AddActorWorldOffset` (`GameplayStatics.GetPlayerCharacter` 0) (0.0 0.0 -10.0) false false)
      (`KismetSystemLibrary.Delay` 0.2)
      (if (`self.qHeld`)
        (goto _label_2))))
  (:`Released`
    (set `self.qHeld` false)))

(fn `UserConstructionScript`
  (bind _top_clif_ref (`self.top clif ref`))
  (bind _bottom_clif_ref (`self.bottom clif ref`))
  (bind (_relativelocation_x _relativelocation_y _relativelocation_z) (`KismetMathLibrary.BreakVector` (`SceneComponent.RelativeLocation` _bottom_clif_ref)))
  (bind (_relativelocation_x_2 _relativelocation_y_2 _relativelocation_z_2) (`KismetMathLibrary.BreakVector` (`SceneComponent.RelativeLocation` _top_clif_ref)))
  (`SceneComponent.K2_SetRelativeLocation` _top_clif_ref (`KismetMathLibrary.MakeVector` (`self.get top clif`) _relativelocation_y_2 _relativelocation_z_2) false false)
  (`SceneComponent.K2_SetRelativeLocation` _bottom_clif_ref (`KismetMathLibrary.MakeVector` (`self.get bottom clif_0`) _relativelocation_y _relativelocation_z) false false))